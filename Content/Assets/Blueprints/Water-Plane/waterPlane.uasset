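; Water plane actor that builds a tiled grid of plane meshes sharing one water material.
; The construction script creates a dynamic material instance from the parent material and applies it to the base plane.
; It writes the referenced light actor's negated forward vector into the material's "Light Direction" parameter.
; Nested TileX/TileY loops add evenly spaced mesh components with the same material, skipping the origin the base plane occupies.
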(fn ConstructionScript
  (bind _reference_to_light_actor (Variables|Default|GetReference%20to%20Light%20Actor))
  (bind _returnvalue (Transformation|GetActorForwardVector _reference_to_light_actor))
  (bind _returnvalue_2 (* _returnvalue -1.0))
  (bind (_x _y _z) (Math|Vector|BreakVector _returnvalue_2))
  (bind _returnvalue_3 (Rendering|Material|CreateDynamicMaterialInstance (Variables|Default|GetParent%20Material%20Instance) "None" "None" :!class /Script/Engine.KismetMaterialLibrary))
  (bind _output_get (Variables|Default|SetMaterialInstance _returnvalue_3))
  (Rendering|Material|SetMaterial (Variables|Default|GetPlane) 0 _output_get)
  (Rendering|Material|SetVectorParameterValue _output_get "Light Direction" (Utilities|Struct|MakeLinearColor _x _y _z 0.0) :!class /Script/Engine.MaterialInstanceDynamic)
  (for _index (range 0 (Variables|Default|GetTile%20X))
    (for _index_2 (range 0 (Variables|Default|GetTile%20Y))
      (if (Math|Boolean|NANDBoolean (== _index 0) (== _index_2 0))
        (bind _returnvalue_4 (AddComponent|AddStaticMeshComponent false (Math|Transform|MakeTransform (Math|Vector|MakeVector (* _index 1e+03) (* _index_2 1e+03) 0.0))))
        (Rendering|Material|SetMaterial _returnvalue_4 0 (Variables|Default|GetMaterialInstance))))))